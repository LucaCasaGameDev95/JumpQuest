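; BP_ArenaDoor is a two-leaf arena door Blueprint that swings open and closed on OnOpenDoors and OnCloseDoors events.
; OnOpenDoors plays the OpenCloseDoor timeline, whose Alpha lerps the relative rotation of Door1 and Door2 from separate start rotations to a shared end rotation along the shortest path.
; OnCloseDoors reverses the same timeline to close both leaves.
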(event Custom|OnOpenDoors
  ;[1 1 1] Open/Close doors
  (bind _alpha (Timeline|OpenCloseDoor Play)
    (:Update
      (Utilities|FlowControl|Sequence
        (:then_0
          (Transformation|SetRelativeRotation (Variables|Default|GetDoor1) (Math|Rotator|Lerp(Rotator) (Variables|Default|GetStartRotationDoor1) (Variables|Default|GetEndRotationDoors) _alpha true) false false))
        (:then_1
          (Transformation|SetRelativeRotation (Variables|Default|GetDoor2) (Math|Rotator|Lerp(Rotator) (Variables|Default|GetStartRotationDoor2) (Variables|Default|GetEndRotationDoors) _alpha true) false false))))))

(event Custom|OnCloseDoors
  ;[1 1 1] Open/Close doors
  (bind _alpha (Timeline|OpenCloseDoor Reverse)
    (:Update
      (Utilities|FlowControl|Sequence
        (:then_0
          (Transformation|SetRelativeRotation (Variables|Default|GetDoor1) (Math|Rotator|Lerp(Rotator) (Variables|Default|GetStartRotationDoor1) (Variables|Default|GetEndRotationDoors) _alpha true) false false))
        (:then_1
          (Transformation|SetRelativeRotation (Variables|Default|GetDoor2) (Math|Rotator|Lerp(Rotator) (Variables|Default|GetStartRotationDoor2) (Variables|Default|GetEndRotationDoors) _alpha true) false false))))))

(fn ConstructionScript)