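; BP_MisteryBox is a breakable mystery box that the player hits from below to release a random collectible.
; When a Player-tagged actor overlaps BreakableCollision, it plays a sound, then calls DropCollectible if the velocity returned through an interface message points upward.
; DropCollectible randomly picks nothing, coin, heart or invulnerability, spawns it above the box and destroys the box.
; Spawned pickups get an upward impulse with random horizontal spread.
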(event OnComponentBeginOverlap(BreakableCollision)
  (params (OverlappedComponent :type Primitive%20Component%20Object%20Reference) (OtherActor :type Actor%20Object%20Reference) (OtherComp :type Primitive%20Component%20Object%20Reference) (OtherBodyIndex :type Integer) (bFromSweep :type Boolean) (SweepResult :type Hit%20Result%20Structure%20%28by%20ref%29))
  ;[1 1 1] Check collision under the box by player
  (if (Actor|ActorHasTag OtherActor "Player")
    ;[1 1 1] sound
    (Audio|PlaySound2D "/Game/Custom/SoundWaves/blocco-rotto-con-testata.blocco-rotto-con-testata" 5.0 1.0 0.25 0 0)
    (bind _velocity (Class|IPlayer|IGetVelocity(Message) OtherActor))
    (if (> (.Z (Class|KismetMathLibrary|BreakVector3f _velocity)) 0.0)
      (CallFunction|DropCollectible))))

(event Custom|DropCollectible
  (bind _misterybox (Variables|Default|GetMisteryBox))
  (bind _returnvalue (Transformation|GetWorldLocation _misterybox))
  (bind _returnvalue_2 (+ _returnvalue "0.000000,0.000000,50.000000"))
  ;[1 1 1] Spawn collectible
  (switch int (Math|Random|RandomIntegerinRange 0 3)
    (:0
      ;;[1 1 1] Nothing
      (Development|PrintString "nothing"))
    (:1
      (Development|PrintString "coin")
      ;;[1 1 1] Coin
      (bind _returnvalue_3 (Game|SpawnActorfromClass "/Game/Custom/Blueprints/BP_NotMandatoryCoin.BP_NotMandatoryCoin_C" (Math|Transform|MakeTransform _returnvalue_2 "0, 0, 0" "1.000000,1.000000,1.000000") "Undefined" "MultiplyWithRoot" 0 false false 0))
      (CallFunction|AddImpulsetoCollectibleSpawned _returnvalue_3))
    (:2
      (Development|PrintString "heart")
      ;;[1 1 1] Heart
      (bind _returnvalue_4 (Game|SpawnActorfromClass "/Game/Custom/Blueprints/BP_Heart.BP_Heart_C" (Math|Transform|MakeTransform _returnvalue_2 "0, 0, 0" "1.000000,1.000000,1.000000") "Undefined" "MultiplyWithRoot" 0 0))
      (CallFunction|AddImpulsetoCollectibleSpawned _returnvalue_4))
    (:3
      (Development|PrintString "invulnerability")
      ;;[1 1 1] Invulnerability
      (bind _returnvalue_5 (Game|SpawnActorfromClass "/Game/Custom/Blueprints/BP_Invulnerability.BP_Invulnerability_C" (Math|Transform|MakeTransform _returnvalue_2 "0, 0, 0" "1.000000,1.000000,1.000000") "Undefined" "MultiplyWithRoot" 0 0))
      (CallFunction|AddImpulsetoCollectibleSpawned _returnvalue_5)))
  ;[1 1 1] destroy mistery box
  (Actor|DestroyActor))

(fn ConstructionScript)

(fn AddImpulsetoCollectibleSpawned
  (params (Mesh :type BP%20Base%20Collectible%20Object%20Reference))
  (bind _returnvalue (Math|Random|RandomFloatinRange 0.0 2e+02))
  (Physics|AddImpulse (Variables|/Game/Custom/Blueprints/BP_BaseCollectible.BP_BaseCollectible_C|GetContainerMesh Mesh) (Math|Vector|MakeVector _returnvalue _returnvalue 5e+02) "None" true)
  (return))