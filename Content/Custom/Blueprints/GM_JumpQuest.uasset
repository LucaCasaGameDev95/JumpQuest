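; GM_JumpQuest, apparently the game mode for JumpQuest, keeps a registry of arenas and tracks which arena handler is active.
; Arenas are added to a list through an event, and a name lookup over that list sets the active handler.
; Player death calls the death dispatcher, then clears any active arena and plays the door-opening sound, which also plays on BeginPlay.
; GetActiveArenaName is a stub returning "None".
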(event Custom|OnPlayerDeath
  ;[1 1 1] Player death dispatcher
  (Default|CallPlayerDeath)
  ;[1 1 1] deactive current arena
  (Utilities|IsValid (Variables|Arenas|GetActiveArenaHandler)
    (:Is%20Valid
      (Variables|Arenas|SetActiveArenaHandler 0)
      ;[1 1 1] open doors sound
      (Audio|PlaySound2D "/Game/Custom/SoundWaves/Appertura_porta.Appertura_porta" 0.6 1.0 0.0 0 0))))

(event Custom|OnSetActiveArena
  (params (ArenaName :type Name))
  ;[1 1 1] OnSetActiveArena
  (for _array_element (Variables|Default|GetArenas)
    (bind _name (Default|GetArenaName _array_element))
    (if (== _name ArenaName)
      (Setter|SetActiveArenaHandler _array_element))))

(event Custom|OnAddArenaToArenasList
  (params (Arena :type BP%20Arena%20Handler%20Object%20Reference))
  ;[1 1 1] Add arena to list
  (Utilities|Array|Add (Variables|Default|GetArenas) Arena))

(event EventBeginPlay
  ;[1 1 1] open doors sound
  (Audio|PlaySound2D "/Game/Custom/SoundWaves/Appertura_porta.Appertura_porta" 0.6 1.0 0.0 0 0))

(fn ConstructionScript)

(fn GetActiveArenaHandler
  (return (Variables|Arenas|GetActiveArenaHandler)))

(fn GetActiveArenaName
  (return "None"))

(fn SetActiveArenaHandler
  (params (ArenaHandler :type BP%20Arena%20Handler%20Object%20Reference))
  (Variables|Arenas|SetActiveArenaHandler ArenaHandler)
  (return))