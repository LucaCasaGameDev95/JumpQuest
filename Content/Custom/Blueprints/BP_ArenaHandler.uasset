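; Arena manager for the JumpQuest game mode that locks the player in until all its enemies are defeated and all coins collected.
; Player overlap makes it the active arena in GM_JumpQuest and closes its doors; completion reopens them and notifies the game mode.
; Coins, floating coins and mystery boxes spawn at placed marker actors and are tracked for reset.
; Reset clears progress, closes doors and respawns those pickups, but not enemies.
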(event OnComponentBeginOverlap(Box)
  (params (OverlappedComponent :type Primitive%20Component%20Object%20Reference) (OtherActor :type Actor%20Object%20Reference) (OtherComp :type Primitive%20Component%20Object%20Reference) (OtherBodyIndex :type Integer) (bFromSweep :type Boolean) (SweepResult :type Hit%20Result%20Structure%20%28by%20ref%29))
  ;[1 1 1] Active arena on overlap
  (if (Actor|ActorHasTag OtherActor "Player")
    (bind _asgm_jump_quest (Utilities|Casting|CastToGM_JumpQuest (Game|GetGameMode)))
    (bind _arenaname (Default|GetActiveArenaName _asgm_jump_quest))
    (if (and (not (Variables|ArenaConfig|GetIsCompleted?)) (!= _arenaname (Variables|ArenaConfig|GetArenaName)))
      (Default|OnSetActiveArena _asgm_jump_quest (Variables|ArenaConfig|GetArenaName))
      (CallFunction|OnCloseDoors))))

(event Custom|OnEnemyDeath
  ;[1 1 1] OnEnemyDeath
  (Math|Integer|IncrementInt (Variables|Enemies|GetEnemyDefeated)
    (:%20%20
      (Utility|CheckifArenaIsCompleted))))

(event Custom|OnCollectibleSpawned
  ;[1 1 1] OnCollectibleSpawned
  (Math|Integer|IncrementInt (Variables|Collectable|GetCollectibleToCollect)))

(event Custom|OnCollectiblePickup
  ;[1 1 1] OnCollectiblePickup
  (Math|Integer|IncrementInt (Variables|Collectable|GetCollectibleCollected)
    (:%20%20
      (Utility|CheckifArenaIsCompleted))))

(event Custom|OnResetArena
  ;[1 1 1] Reset Arena
  ;;[1 1 1] Arena config and doors
  (Utility|ResetArenaConfig)
  (CallFunction|OnCloseDoors)
  ;;[1 1 1] Reset coins
  (Collectibles|DestroyAllCollectibleReferences)
  (Collectibles|SpawnInitialCoins)
  (Collectibles|SpawnInitialFloatingCoins)
  ;;[1 1 1] reset mystery boxes
  (Collectibles|DestroyAllMisteryBoxesReferences)
  (Collectibles|SpawnInitialMysteryBoxes))

(event Custom|OnOpenDoors
  ;[1 1 1] Open/Close arena doors
  (for _array_element (Variables|Doors|GetArenaDoors)
    (Default|OnOpenDoors _array_element)))

(event Custom|OnCloseDoors
  ;[1 1 1] Open/Close arena doors
  (for _array_element (Variables|Doors|GetArenaDoors)
    (Default|OnCloseDoors _array_element)))

(event EventBeginPlay
  ;[1 1 1] Begin play
  (Utilities|FlowControl|Sequence
    (:then_0
      ;;[1 1 1] Bind to enemy death
      (for _array_element (Variables|Enemies|GetEnemyToDefeat)
        (EventDispatchers|BindEventtoEnemyDeath _array_element (EventDispatchers|CreateEvent :!event Custom|OnEnemyDeath))))
    (:then_1
      ;;[1 1 1] Bind to player death
      (bind _asgm_jump_quest (Utilities|Casting|CastToGM_JumpQuest (Game|GetGameMode)))
      (EventDispatchers|BindEventtoPlayerDeath _asgm_jump_quest (EventDispatchers|CreateEvent :!event Custom|OnResetArena)))
    (:then_2
      ;;[1 1 1] Add arena to GM list
      (bind _asgm_jump_quest_2 (Utilities|Casting|CastToGM_JumpQuest (Game|GetGameMode)))
      (Default|OnAddArenatoArenasList _asgm_jump_quest_2 self))
    (:then_3
      ;;[1 1 1] Spawn initial coins
      (Collectibles|SpawnInitialCoins)
      (Collectibles|SpawnInitialFloatingCoins))
    (:then_4
      ;;[1 1 1] Spawn initial mistery boxes
      (Collectibles|SpawnInitialMysteryBoxes))))

(fn ConstructionScript)

(fn ResetArenaConfig
  (Variables|Enemies|SetEnemyDefeated 0)
  (Variables|Collectable|SetCollectibleCollected 0)
  (Variables|Collectable|SetCollectibleToCollect 0)
  (Variables|ArenaConfig|SetIsCompleted? false))

(fn CheckifArenaIsCompleted
  (if (Math|Boolean|ANDBoolean (== (Variables|Collectable|GetCollectibleCollected) (Variables|Collectable|GetCollectibleToCollect)) (== (Variables|Enemies|GetEnemyDefeated) (Utilities|Array|Length (Variables|Enemies|GetEnemyToDefeat))) (not (Variables|ArenaConfig|GetIsCompleted?)))
    (Development|PrintString "Arena completata")
    ;[1 1 1] Open door and complete arena
    (CallFunction|OnOpenDoors)
    (Variables|ArenaConfig|SetIsCompleted? true)
    (bind _asgm_jump_quest (Utilities|Casting|CastToGM_JumpQuest (Game|GetGameMode)))
    (Default|SetActiveArenaHandler _asgm_jump_quest)
    (return)
    (else
      (Development|PrintString "Aerna NON completata"))))

(fn GetArenaName
  (return (Variables|ArenaConfig|GetArenaName)))

(fn SpawnInitialCoins
  (bind _arenacoins (Variables|Collectable|GetArenaCoins))
  (for _array_element _arenacoins
    (bind _returnvalue (Game|SpawnActorfromClass "/Game/Custom/Blueprints/BP_Coin.BP_Coin_C" (Math|Transform|MakeTransform (Transformation|GetActorLocation _array_element) "0, 0, 0" "1.000000,1.000000,1.000000") "Undefined" "MultiplyWithRoot" 0 false true 0))
    (Utilities|Array|Add (Variables|Collectable|GetCollectibleReferences) _returnvalue))
  (Variables|Collectable|SetCollectibleToCollect (+ (Utilities|Array|Length _arenacoins) (Variables|Collectable|GetCollectibleToCollect))))

(fn DestroyAllMisteryBoxesReferences
  (for _array_element (Variables|Collectable|GetMysteryBoxesReferences)
    (Utilities|IsValid _array_element
      (:Is%20Valid
        (Actor|DestroyActor _array_element))))
  (Utilities|Array|Clear (Variables|Collectable|GetMysteryBoxesReferences)))

(fn SpawnInitialMysteryBoxes
  (for _array_element (Variables|Collectable|GetArenaMysteryBoxes)
    (bind _returnvalue (Game|SpawnActorfromClass "/Game/Custom/Blueprints/BP_MisteryBox.BP_MisteryBox_C" (Math|Transform|MakeTransform (Transformation|GetActorLocation _array_element) "0, 0, 0" "1.000000,1.000000,1.000000") "Undefined" "MultiplyWithRoot" 0 0))
    (Utilities|Array|Add (Variables|Collectable|GetMysteryBoxesReferences) _returnvalue)))

(fn SpawnInitialFloatingCoins
  (bind _arenafloatingcoins (Variables|Collectable|GetArenaFloatingCoins))
  (for _array_element _arenafloatingcoins
    (bind _returnvalue (Game|SpawnActorfromClass "/Game/Custom/Blueprints/BP_Coin.BP_Coin_C" (Math|Transform|MakeTransform (Transformation|GetActorLocation _array_element) "0, 0, 0" "1.000000,1.000000,1.000000") "Undefined" "MultiplyWithRoot" 0 true true 0))
    (Utilities|Array|Add (Variables|Collectable|GetCollectibleReferences) _returnvalue))
  (Variables|Collectable|SetCollectibleToCollect (+ (Utilities|Array|Length _arenafloatingcoins) (Variables|Collectable|GetCollectibleToCollect))))

(fn DestroyAllCollectibleReferences
  (for _array_element (Variables|Collectable|GetCollectibleReferences)
    (Utilities|IsValid _array_element
      (:Is%20Valid
        (Actor|DestroyActor _array_element))))
  (Utilities|Array|Clear (Variables|Collectable|GetCollectibleReferences)))