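; Base collectible actor for JumpQuest that the player picks up by overlap and that reports to the active arena.
; On BeginPlay it fetches the active arena handler from GM_JumpQuest and, if valid, notifies it of the spawn.
; A Player-tagged overlap on ContainerCollision notifies the current handler, fires the empty OnCollectiblePickup hook, then destroys the actor.
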(event OnComponentBeginOverlap(ContainerCollision)
  (params (OverlappedComponent :type Primitive%20Component%20Object%20Reference) (OtherActor :type Actor%20Object%20Reference) (OtherComp :type Primitive%20Component%20Object%20Reference) (OtherBodyIndex :type Integer) (bFromSweep :type Boolean) (SweepResult :type Hit%20Result%20Structure%20%28by%20ref%29))
  ;[1 1 1] Pickup collected
  (if (Actor|ActorHasTag OtherActor "Player")
    (bind _asgm_jump_quest (Utilities|Casting|CastToGM_JumpQuest (Game|GetGameMode)))
    (bind _arena (Default|GetActiveArenaHandler _asgm_jump_quest))
    (Utilities|IsValid _arena
      (:Is%20Valid
        (Default|OnCollectiblePickup _arena))
      (:Is%20Not%20Valid
        _))
    (CallFunction|OnCollectiblePickup)
    (Actor|DestroyActor)))

(event Custom|OnCollectiblePickup
  ;[1 1 1] Collectible pickup
)

(event EventBeginPlay
  ;[1 1 1] Tell active arena that has spawnde new collectible (if spawn with arena active)
  (bind _asgm_jump_quest (Utilities|Casting|CastToGM_JumpQuest (Game|GetGameMode)))
  (bind _arena (Default|GetActiveArenaHandler _asgm_jump_quest))
  (Utilities|IsValid _arena
    (:Is%20Valid
      (Default|OnCollectibleSpawned _arena))))

(fn ConstructionScript)