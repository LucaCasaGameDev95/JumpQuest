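; BP_Shooter is a shooter enemy Blueprint that supplies patrol destinations and leaves BeginPlay and construction to its parent class.
; GetNextPatrolPosition increments an index into the patrol target points, wrapping to zero at the end of the array.
; It returns that point actor's location, or the shooter's own location when the entry is invalid.
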(event EventBeginPlay
  (|CallParentFunction))

(fn ConstructionScript
  (|CallParentFunction))

(fn GetNextPatrolPosition
  (bind _result (Math|Integer|IncrementInt (Variables|Default|GetCurrentPatrolTargetPointIndex))
    (:%20%20
      (if (>= _result (Utilities|Array|Length (Variables|Default|GetPatrolTargetPoints)))
        (Variables|Default|SetCurrentPatrolTargetPointIndex 0))
      (Utilities|IsValid (Utilities|Array|Get(acopy) (Variables|Default|GetPatrolTargetPoints) (Variables|Default|GetCurrentPatrolTargetPointIndex))
        (:Is%20Valid
          (return (Transformation|GetActorLocation (Utilities|Array|Get(acopy) (Variables|Default|GetPatrolTargetPoints) (Variables|Default|GetCurrentPatrolTargetPointIndex)))))
        (:Is%20Not%20Valid
          (return (Transformation|GetActorLocation)))))))