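; AI controller for shooter enemies that runs a patrol, chase and attack behavior tree on possession.
; Sight perception of Player-tagged actors sets line-of-sight and target blackboard keys, clearing them after a grace timer once sight is lost.
; While a target is tracked, a looping timer compares distance to the shooting range and updates the ranged-attack key, which a separate event can reset.
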(event OnTargetPerceptionUpdated(AIPerception)
  (params (Actor :type Actor%20Object%20Reference) (Stimulus :type AI%20Stimulus%20Structure))
  (bind _blackboard (Variables|Default|GetBlackboard))
  ;[1 1 1] Player?
  (if (Actor|ActorHasTag Actor "Player")
    (Variables|Default|SetPerceivedActor Actor)
    (bind _returnvalue (Class|AIPerceptionSystem|GetSenseClassforStimulus Stimulus))
    (if (== _returnvalue "/Script/AIModule.AISense_Sight")
      (if (.bSuccessfullySensed (Utilities|Struct|BreakAIStimulus Stimulus))
        ;[1 1 1] Invalidate timer
        (Utilities|Time|ClearandInvalidateTimerbyHandle (Variables|Default|GetLineOfSightTimer))
        ;[1 1 1] Set LineOfSight
        (AI|Components|Blackboard|SetValueasBool _blackboard (Utilities|Name|MakeLiteralName "HasLineOfSight") true)
        (AI|Components|Blackboard|SetValueasObject _blackboard (Utilities|Name|MakeLiteralName "TargetActor") (Variables|Default|GetPerceivedActor))
        (bind _returnvalue_2 (Utilities|Time|SetTimerbyEvent (delegate Custom|CheckAttackRanged) 1.0 true))
        (Variables|Default|SetAttackTimer _returnvalue_2)
        (else
          ;[1 1 1] Wait while chase and recheck
          (bind _returnvalue_3 (Utilities|Time|SetTimerbyEvent (delegate Custom|OnStartTimer) (Variables|Default|GetLineOfSightDuration)))
          (Variables|Default|SetLineOfSightTimer _returnvalue_3))))))

(event Custom|OnStartTimer
  (bind _blackboard (Variables|Default|GetBlackboard))
  ;[1 1 1] Wait while chase and recheck
  (AI|Components|Blackboard|SetValueasBool _blackboard (Utilities|Name|MakeLiteralName "HasLineOfSight") false)
  (AI|Components|Blackboard|SetValueasObject _blackboard (Utilities|Name|MakeLiteralName "TargetActor") 0)
  (Utilities|Time|ClearandInvalidateTimerbyHandle (Variables|Default|GetAttackTimer)))

(event Custom|CheckAttackRanged
  ;[1 1 1] Can range attack?
  (if (<= (Math|Vector|Distance(Vector) (Transformation|GetActorLocation (Variables|Default|GetPossessed%20Pawn)) (Transformation|GetActorLocation (Variables|Default|GetPerceivedActor))) (Variables|Default|GetDistanceToShoot))
    (AI|Components|Blackboard|SetValueasBool (Variables|Default|GetBlackboard) (Utilities|Name|MakeLiteralName "CanRangeAttack?") true)
    (else
      (AI|Components|Blackboard|SetValueasBool (Variables|Default|GetBlackboard) (Utilities|Name|MakeLiteralName "CanRangeAttack?") false))))

(event Custom|ResetRangeAttack
  ;[1 1 1] Can range attack?
  (AI|Components|Blackboard|SetValueasBool (Variables|Default|GetBlackboard) (Utilities|Name|MakeLiteralName "CanRangeAttack?") false))

(event EventPossess
  (params (PossessedPawn :type Pawn%20Object%20Reference))
  ;[1 1 1] Active behaviour tree
  (Variables|Default|SetPossessed%20Pawn PossessedPawn)
  (AI|RunBehaviorTree "/Game/Characters/Enemies/Shooter/AI/BT_PatrolChaseAndAttack.BT_PatrolChaseAndAttack"))

(fn ConstructionScript)