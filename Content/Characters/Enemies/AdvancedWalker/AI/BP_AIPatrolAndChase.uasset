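; AI controller for a patrol-and-chase enemy that runs BT_PatrolAndChase on the pawn it possesses.
; Sight perception of actors tagged Player sets the HasLineOfSight and TargetActor blackboard keys for the tree.
; When sight is lost, a LineOfSightDuration timer delays clearing both keys, so the chase continues briefly unless re-sighting cancels the timer.
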(event OnTargetPerceptionUpdated(AIPerception)
  (params (Actor :type Actor%20Object%20Reference) (Stimulus :type AI%20Stimulus%20Structure))
  (bind _blackboard (Variables|Default|GetBlackboard))
  ;[1 1 1] Player?
  (if (Actor|ActorHasTag Actor "Player")
    (Variables|Default|SetTarget Actor)
    (bind _returnvalue (Class|AIPerceptionSystem|GetSenseClassforStimulus Stimulus))
    (if (== _returnvalue "/Script/AIModule.AISense_Sight")
      (if (.bSuccessfullySensed (Utilities|Struct|BreakAIStimulus Stimulus))
        ;[1 1 1] Invalidate timer
        (Utilities|Time|ClearandInvalidateTimerbyHandle (Variables|Default|GetLineOfSightTimer))
        ;[1 1 1] Set LineOfSight
        (AI|Components|Blackboard|SetValueasBool _blackboard (Utilities|Name|MakeLiteralName "HasLineOfSight") true)
        (AI|Components|Blackboard|SetValueasObject _blackboard (Utilities|Name|MakeLiteralName "TargetActor") (Variables|Default|GetTarget))
        (else
          ;[1 1 1] Wait while chase and recheck
          (bind _returnvalue_2 (Utilities|Time|SetTimerbyEvent (delegate Custom|OnStartTimer) (Variables|Default|GetLineOfSightDuration)))
          (Variables|Default|SetLineOfSightTimer _returnvalue_2))))))

(event Custom|OnStartTimer
  (bind _blackboard (Variables|Default|GetBlackboard))
  ;[1 1 1] Wait while chase and recheck
  (AI|Components|Blackboard|SetValueasBool _blackboard (Utilities|Name|MakeLiteralName "HasLineOfSight") false)
  (AI|Components|Blackboard|SetValueasObject _blackboard (Utilities|Name|MakeLiteralName "TargetActor") 0))

(event EventPossess
  (params (PossessedPawn :type Pawn%20Object%20Reference))
  ;[1 1 1] Active behaviour tree
  (Variables|Default|SetPossessed%20Pawn PossessedPawn)
  (AI|RunBehaviorTree "/Game/Characters/Enemies/AdvancedWalker/AI/BT_PatrolAndChase.BT_PatrolAndChase"))

(fn ConstructionScript)