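; BP_SimpleWalker is an enemy NPC that starts patrolling an array of patrol points on BeginPlay.
; OnMoveNPC picks a random navigable location within a radius of the current point and sends the pawn there with AI MoveTo.
; Success waits briefly and failure barely pauses before both advance the wrapping index and call the event again.
; An invalid point ends the loop, while a failed location query retries immediately.
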(event Custom|OnMoveNPC
  ;[1 1 1] Move trough target points
  (Utilities|IsValid (Utilities|Array|Get(acopy) (Variables|Default|GetPatrolPoints) (Variables|Default|GetcurrentPatrolPointIndex))
    (:Is%20Valid
      (bind _output_get (Variables|Default|SetCurrentPatrolPointTarget (Utilities|Array|Get(acopy) (Variables|Default|GetPatrolPoints) (Variables|Default|GetcurrentPatrolPointIndex))))
      (bind (_randomlocation _returnvalue) (Class|NavigationSystemV1|GetRandomLocationinNavigableRadius (Transformation|GetActorLocation _output_get) (Variables|Default|GetRadius) (Variables|Default|GetNavigationMesh) 0))
      (if _returnvalue
        (AI|AIMoveTo self _randomlocation 0 5.0 false
          (:OnSuccess
            (Utilities|FlowControl|Delay 3.0))
          (:OnFail
            (Utilities|FlowControl|Delay 0.1)))
        (if (== (+ (Variables|Default|GetcurrentPatrolPointIndex) 1) (Utilities|Array|Length (Variables|Default|GetPatrolPoints)))
          (Variables|Default|SetcurrentPatrolPointIndex 0)
          (else
            (Math|Integer|IncrementInt (Variables|Default|GetcurrentPatrolPointIndex)
              (:%20%20
                _))))
        (CallFunction|OnMoveNPC)
        (else
          (CallFunction|OnMoveNPC))))))

(event EventBeginPlay
  ;[1 1 1] Start moving
  (|CallParentFunction)
  (CallFunction|OnMoveNPC))

(fn ConstructionScript)