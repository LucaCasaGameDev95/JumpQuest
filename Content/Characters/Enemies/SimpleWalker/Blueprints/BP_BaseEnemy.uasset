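; BP_BaseEnemy is an enemy character that hurts the player on contact and dies when stomped from above.
; Overlapping its capsule sends a damage interface message to any actor tagged Player.
; A separate head collider reads the player's velocity through an interface and, if it is falling, calls EnemyDeath and destroys the enemy.
; BeginPlay sets a fixed walk speed, with no movement logic in this graph.
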(event OnComponentBeginOverlap(EnemyCapsuleComponent)
  (params (OverlappedComponent :type Primitive%20Component%20Object%20Reference) (OtherActor :type Actor%20Object%20Reference) (OtherComp :type Primitive%20Component%20Object%20Reference) (OtherBodyIndex :type Integer) (bFromSweep :type Boolean) (SweepResult :type Hit%20Result%20Structure%20%28by%20ref%29))
  ;[1 1 1] Take damage if touch player
  (if (Actor|ActorHasTag OtherActor "Player")
    (Class|IPlayer|ITakeDamage(Message) OtherActor 1.0)))

(event OnComponentBeginOverlap(EnemyHead)
  (params (OverlappedComponent :type Primitive%20Component%20Object%20Reference) (OtherActor :type Actor%20Object%20Reference) (OtherComp :type Primitive%20Component%20Object%20Reference) (OtherBodyIndex :type Integer) (bFromSweep :type Boolean) (SweepResult :type Hit%20Result%20Structure%20%28by%20ref%29))
  ;[1 1 1] Death if player jump on my head
  (if (Actor|ActorHasTag OtherActor "Player")
    (bind _velocity (Class|IPlayer|IGetVelocity(Message) OtherActor))
    (if (< (.Z (Class|KismetMathLibrary|BreakVector3f _velocity)) 0.0)
      (Default|CallEnemyDeath)
      (Actor|DestroyActor))))

(event EventBeginPlay
  ;[1 1 1] Set base speed
  (Variables|/Script/Engine.CharacterMovementComponent|SetMaxWalkSpeed (Variables|Character|GetCharacterMovement) 2e+02))

(fn ConstructionScript)